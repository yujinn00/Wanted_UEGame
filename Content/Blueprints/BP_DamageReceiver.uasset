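; BP_DamageReceiver tracks health, handling damage, healing and death, with health set to maximum on BeginPlay.
; ReceiveDamage subtracts damage and, at zero or below, sets health to zero and fires OnDead.
; GainHealthPower clamps healing between zero and maximum and fires OnHealthPowerChanged, which the damage path does not fire.
; GetHPPercent returns current health as a fraction of maximum.
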(event Custom|ReceiveDamage
  (params (Damage :type Float%20%28double-precision%29))
  ;[1 1 1] 데미지 처리 공식
  (Variables|Default|SetHealthPower (- (Variables|Default|GetHealthPower) Damage))
  ;[1 1 1] 사망 처리
  (if (<= (Variables|Default|GetHealthPower) 0.0)
    (Variables|Default|SetHealthPower 0.0)
    (Default|CallOnDead)))

(event Custom|GainHealthPower
  (params (GainAmount :type Float%20%28double-precision%29))
  (Variables|Default|SetHealthPower (Math|Float|Clamp(Float) (+ (Variables|Default|GetHealthPower) GainAmount) 0.0 (Variables|Default|GetMaxHealthPower)))
  (Default|CallOnHealthPowerChanged))

(event EventBeginPlay
  ;[1 1 1] 초기화
  (Variables|Default|SetHealthPower (Variables|Default|GetMaxHealthPower)))

(fn GetHPPercent
  (return (/ (Variables|Default|GetHealthPower) (Variables|Default|GetMaxHealthPower))))