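; Bear monster enemy that spots, chases and attacks the BP_Warrior player until either dies or the player leaves sight radius.
; A state enum sets walk speed and is mirrored to the AI Blackboard; PawnSensing starts chases, Tick ends them.
; AttackCheckBegin/End toggle the damaging attack collision.
; Damage feeds DamageReceiver, HP widget, camera shake and timeline-driven material flash; death plays a dissolve before destroying the actor.
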(event OnSeePawn(PawnSensing)
  (params (Pawn :type Pawn%20Object%20Reference))
  ;[1 1 1] 플레이어 감지 및 추적
  (if (Utilities|Enum|Equal(Enum) (Variables|Default|GetState) "NewEnumerator0")
    (bind _asbp_warrior (Utilities|Casting|CastToBP_Warrior Pawn))
    (if (Utilities|Enum|NotEqual(Enum) (Variables|/Game/Blueprints/Warrior/BP_Warrior.BP_Warrior_C|GetState _asbp_warrior) "NewEnumerator2")
      (CallFunction|SetState "NewEnumerator1")
      (bind _output_get (Variables|Actor|SetInstigator Pawn))
      (AI|Components|Blackboard|SetValueasObject (Variables|/Script/AIModule.AIController|GetBlackboard (AI|GetAIController self)) (Variables|Default|GetTargetPlayerKey) _output_get))))

(event OnComponentBeginOverlap(AttackCollision)
  (params (OverlappedComponent :type Primitive%20Component%20Object%20Reference) (OtherActor :type Actor%20Object%20Reference) (OtherComp :type Primitive%20Component%20Object%20Reference) (OtherBodyIndex :type Integer) (bFromSweep :type Boolean) (SweepResult :type Hit%20Result%20Structure%20%28by%20ref%29))
  ;[1 1 1] 데미지 적용
  (Game|Damage|ApplyDamage OtherActor (Variables|Default|GetDamage) (Pawn|GetController) self))

(event Custom|SetState
  (params (NewState :type E_BearState%20Enum :default "NewEnumerator0"))
  ;[1 1 1] 몬스터 상태 변경
  (if (Utilities|Enum|NotEqual(Enum) (Variables|Default|GetState) "NewEnumerator3")
    (if (Utilities|Enum|NotEqual(Enum) (Variables|Default|GetState) NewState)
      (bind _output_get (Variables|Default|SetState NewState))
      (AI|Components|Blackboard|SetValueasEnum (AI|GetBlackboard (AI|GetAIController self)) (Variables|Default|GetStateKey) _output_get)
      (Utilities|FlowControl|Sequence ; 순차적으로 실행해주는 편의 노드
        (:then_0
          (switch Utilities|FlowControl|Switch|SwitchonE_BearState (Variables|Default|GetState)
            (:NewEnumerator0
              (Variables|/Script/Engine.CharacterMovementComponent|SetMaxWalkSpeed (Variables|Character|GetCharacterMovement) 2e+02))
            (:NewEnumerator1
              (Variables|/Script/Engine.CharacterMovementComponent|SetMaxWalkSpeed (Variables|Character|GetCharacterMovement) 5e+02))
            (:NewEnumerator2
              (Variables|/Script/Engine.CharacterMovementComponent|SetMaxWalkSpeed (Variables|Character|GetCharacterMovement) 0.0 :!label _label))
            (:NewEnumerator3
              (goto _label))))))))

(event Custom|OnChase
  ;[1 1 1] 플레이어 추적
  (Utilities|IsValid (Variables|Actor|GetInstigator)
    (:Is%20Valid
      (if (> (Math|Vector|Distance(Vector) (Transformation|GetActorLocation (Variables|Actor|GetInstigator)) (Transformation|GetActorLocation)) (Variables|/Script/AIModule.PawnSensingComponent|GetSightRadius (Variables|Default|GetPawnSensing)))
        (Variables|Actor|SetInstigator 0)
        (CallFunction|SetState "NewEnumerator0")))))

(event Custom|OnDead
  ;[1 1 1] 초기화
  (CallFunction|SetState "NewEnumerator3")
  (Collision|SetCollisionEnabled (Variables|Collision|GetCapsuleComponent) "NoCollision")
  (bind (_direction _dissolve _dissolvecolor) (Timeline|DeadEvent Play)
    (:Update
      (Rendering|Material|SetScalarParameterValue (Variables|Default|GetDynamicInstance) "Dissolve" _dissolve :!class /Script/Engine.MaterialInstanceDynamic)
      (Rendering|Material|SetScalarParameterValue (Variables|Default|GetDynamicInstance) "HitValue" (* _dissolve 1e+02) :!class /Script/Engine.MaterialInstanceDynamic)
      (Rendering|Material|SetVectorParameterValue (Variables|Default|GetDynamicInstance) "HitColor" _dissolvecolor :!class /Script/Engine.MaterialInstanceDynamic))
    (:Finished
      (Actor|DestroyActor))))

(event Custom|OnAttack
  ;[1 1 1] 플레이어 사망 시 공격 중지 처리
  (Utilities|IsValid (Variables|Actor|GetInstigator)
    (:Is%20Valid
      (bind _asbp_warrior (Utilities|Casting|CastToBP_Warrior (Variables|Actor|GetInstigator)))
      (bind _isdead (Default|IsDead _asbp_warrior))
      (if _isdead
        (CallFunction|SetState "NewEnumerator0")
        (Variables|Actor|SetInstigator 0)))))

(event Custom|AttackCheckEnd
  ;[1 1 1] 공격 판정 종료 처리
  (Collision|SetCollisionEnabled (Variables|Default|GetAttackCollision) "NoCollision"))

(event Custom|AttackCheckBegin
  ;[1 1 1] 공격 판정 시작 처리
  (Collision|SetCollisionEnabled (Variables|Default|GetAttackCollision) "QueryOnly"))

(event Custom|OnLocomotion)

(event EventBeginPlay
  ;[1 1 1] 초기화
  (Rendering|SetCastShadow (Variables|Default|GetHPBar) false)
  (bind _returnvalue (Rendering|Material|CreateDynamicMaterialInstance (Variables|Character|GetMesh) 0 "/Game/InfinityBladeAdversaries/Enemy/Enemy_Bear/Materials/M_Bear_Stone_Inst.M_Bear_Stone_Inst" "None" :!class /Script/Engine.PrimitiveComponent))
  (Variables|Default|SetDynamicInstance _returnvalue)
  (EventDispatchers|BindEventtoOnDead (Variables|Default|GetDamageReceiver) (delegate Custom|OnDead))
  (bind _aswbp_hphud (Utilities|Casting|CastToWBP_HPHUD (UserInterface|GetUserWidgetObject (Variables|Default|GetHPBar))))
  (Variables|Default|SetHPHUD _aswbp_hphud)
  (Collision|SetCollisionEnabled (Variables|Default|GetAttackCollision) "NoCollision"))

(event EventTick
  (params (DeltaSeconds :type Float%20%28single-precision%29))
  ;[1 1 1] 몬스터 상태 변경
  (switch Utilities|FlowControl|Switch|SwitchonE_BearState (Variables|Default|GetState)
    (:NewEnumerator0
      (CallFunction|OnLocomotion))
    (:NewEnumerator1
      (CallFunction|OnChase))
    (:NewEnumerator2
      (CallFunction|OnAttack))))

(event Game|Damage|EventAnyDamage
  (params (Damage :type Float%20%28single-precision%29) (DamageType :type Damage%20Type%20Object%20Reference) (InstigatedBy :type Controller%20Object%20Reference) (DamageCauser :type Actor%20Object%20Reference))
  (bind _hphud (Variables|Default|GetHPHUD))
  ;[1 1 1] 피격 처리
  (Default|ReceiveDamage (Variables|Default|GetDamageReceiver) Damage)
  (Default|SetHPPercent _hphud (Default|GetHPPercent (Variables|Default|GetDamageReceiver)))
  (Default|PlayTextAnimation _hphud (Math|Float|Truncate Damage))
  (CameraShakes|StartCameraShake (Game|GetPlayerCameraManager 0) "/Game/Blueprints/Warrior/BP_Shake.BP_Shake_C" 0.1 "CameraLocal" "0, 0, 0")
  (bind _effectvalue (Timeline|HitEffect PlayFromStart)
    (:Update
      (Rendering|Material|SetScalarParameterValue (Variables|Default|GetDynamicInstance) "HitValue" _effectvalue :!class /Script/Engine.MaterialInstanceDynamic))))

(fn ConstructionScript)