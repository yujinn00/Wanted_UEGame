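; BP_Weapon is a pickup weapon that gives BP_Warrior melee and radial attacks.
; Overlapping its Sphere hands the weapon to the warrior, disables the pickup collision and binds RadialAttack to the warrior's radial attack event.
; AttackCollision deals damage on overlap and is query-enabled only between attack check begin and end events.
; RadialAttack applies area damage from the weapon's location, ignoring the player pawn and using a custom damage-prevention channel.
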(event OnComponentBeginOverlap(Sphere)
  (params (OverlappedComponent :type Primitive%20Component%20Object%20Reference) (OtherActor :type Actor%20Object%20Reference) (OtherComp :type Primitive%20Component%20Object%20Reference) (OtherBodyIndex :type Integer) (bFromSweep :type Boolean) (SweepResult :type Hit%20Result%20Structure%20%28by%20ref%29))
  ;[1 1 1] 무기 획득 처리
  (bind _asbp_warrior (Utilities|Casting|CastToBP_Warrior OtherActor))
  (Default|OnWeaponCollected _asbp_warrior self)
  (Collision|SetCollisionEnabled (Variables|Default|GetSphere) "NoCollision")
  (EventDispatchers|BindEventtoRadialAttackEvent _asbp_warrior (delegate Custom|RadialAttack)))

(event OnComponentBeginOverlap(AttackCollision)
  (params (OverlappedComponent :type Primitive%20Component%20Object%20Reference) (OtherActor :type Actor%20Object%20Reference) (OtherComp :type Primitive%20Component%20Object%20Reference) (OtherBodyIndex :type Integer) (bFromSweep :type Boolean) (SweepResult :type Hit%20Result%20Structure%20%28by%20ref%29))
  ;[1 1 1] 데미지 적용 처리
  (Game|Damage|ApplyDamage OtherActor (Variables|Default|GetDamage) (Game|GetPlayerController 0) self))

(event Custom|OnAttackCheckBegin
  ;[1 1 1] 콜리전 적용 처리
  (Collision|SetCollisionEnabled (Variables|Default|GetAttackCollision) "QueryOnly"))

(event Custom|OnAttackCheckEnd
  ;[1 1 1] 콜리전 해제 처리
  (Collision|SetCollisionEnabled (Variables|Default|GetAttackCollision) "NoCollision"))

(event Custom|RadialAttack
  ;[1 1 1] 무기 획득 처리
  (Game|Damage|ApplyRadialDamage (Variables|Default|GetRadialDamage) (Transformation|GetActorLocation) (Variables|Default|GetRadialDamageRadius) 0 (Utilities|Array|MakeArray (Game|Player|GetPlayerPawn 0)) self (Game|GetPlayerController 0) false "ECC_GameTraceChannel4"))

(event EventBeginPlay
  ;[1 1 1] 초기화
  (Collision|SetCollisionEnabled (Variables|Default|GetAttackCollision) "NoCollision"))

(fn ConstructionScript)