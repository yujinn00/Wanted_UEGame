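; BP_Item is a destructible prop that can restore health to the warrior who destroys it.
; AnyDamage subtracts damage from HealthPower; at zero or below, it casts the damage causer's owner to BP_Warrior and, on success, calls GainHealthPower on its DamageReceiver with GainAmount.
; The item then runs Die whether or not the cast succeeds, destroying itself and spawning an explosion emitter at its location.
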(event Custom|Die
  ;[1 1 1] 아이템 삭제 처리
  (Actor|DestroyActor)
  (Effects|SpawnEmitteratLocation "/Game/Particles/P_Explosion.P_Explosion" (Transformation|GetActorLocation)))

(event EventBeginPlay)

(event Collision|EventActorBeginOverlap
  (params (OtherActor :type Actor%20Object%20Reference)))

(event EventTick
  (params (DeltaSeconds :type Float%20%28single-precision%29)))

(event Game|Damage|EventAnyDamage
  (params (Damage :type Float%20%28single-precision%29) (DamageType :type Damage%20Type%20Object%20Reference) (InstigatedBy :type Controller%20Object%20Reference) (DamageCauser :type Actor%20Object%20Reference))
  ;[1 1 1] 아이템 피격 처리
  (bind _output_get (Variables|Default|SetHealthPower (- (Variables|Default|GetHealthPower) Damage)))
  (if (<= _output_get 0.0)
    (bind _asbp_warrior (Utilities|Casting|CastToBP_Warrior (Components|GetOwner DamageCauser))
      (:then
        (Default|GainHealthPower (Variables|/Game/Blueprints/Warrior/BP_Warrior.BP_Warrior_C|GetDamageReceiver _asbp_warrior) (Variables|Default|GetGainAmount))
        (CallFunction|Die))
      (:CastFailed
        (CallFunction|Die)))))

(fn ConstructionScript)